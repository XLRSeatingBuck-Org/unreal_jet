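; BP_TakeoffSetup1 is a Blueprint that switches between three cameras: CamPancake, CamVr and BackCamera.
; On IA_ChangeCamera Started, it deactivates the camera at CamIndex, advances the index with wrap-around, activates the new camera and prints the index.
; Cycling only runs forward, as a constant true condition leaves the alternative index branch unused.
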(event Input|EnhancedActionEvents|EnhancedInputActionIA_ChangeCamera
  (params (ActionValue :type Boolean) (ElapsedSeconds :type Float%20%28double-precision%29) (TriggeredSeconds :type Float%20%28double-precision%29) (InputAction :type Input%20Action%20Object%20Reference :default "/Game/Input/IA_ChangeCamera.IA_ChangeCamera"))
  ;[1 1 1] Current camera deactivated. Iterate to the next item in the list of available cameras. Will go backwards when this is all written in cpp. Blueprint too messy
  (:Started
    (Components|Activation|Deactivate (Utilities|Array|Get(acopy) (Utilities|Array|MakeArray (Variables|Default|Getcam_pancake) (Variables|Default|Getcam_vr) (Variables|Default|GetbackCamera)) (Variables|Default|GetcamIndex)))
    (if (== (Variables|Default|GetcamIndex) 2)
      (Variables|Default|SetcamIndex 0)
      (elif true
        (Variables|Default|SetcamIndex (+ (Variables|Default|GetcamIndex) 1))
        (else
          (Variables|Default|SetcamIndex 2))))
    (Components|Activation|Activate (Utilities|Array|Get(acopy) (Utilities|Array|MakeArray (Variables|Default|Getcam_pancake) (Variables|Default|Getcam_vr) (Variables|Default|GetbackCamera)) (Variables|Default|GetcamIndex)) true)
    (Development|PrintString (Utilities|String|ToString(Integer) (Variables|Default|GetcamIndex)))))

(fn ConstructionScript)